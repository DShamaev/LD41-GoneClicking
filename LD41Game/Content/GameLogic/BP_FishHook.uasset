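; BP_FishHook is a fishing hook actor that travels vertically down to a bottom limit and back up.
; UpdateMovement steps Z by Speed in the current direction and passes the new location to MoveInternally; the actor's own Tick is unused.
; MoveInternally switches to rising at BottomLimit and applies positions below TopLimit.
; At or above TopLimit, it skips the move and clears HookActivated on LD41PlayerController.
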(event EventBeginPlay)

(event Collision|EventActorBeginOverlap
  (params (OtherActor :type Actor%20Object%20Reference)))

(event EventTick
  (params (DeltaSeconds :type Float%20%28single-precision%29)))

(fn ConstructionScript)

(fn UpdateMovement
  (bind _returnvalue (Transformation|GetActorLocation))
  (bind _speed (Variables|Default|Getspeed))
  (bind (_x _y _z) (Math|Vector|BreakVector _returnvalue))
  (bind _returnvalue_2 (- _z _speed))
  (bind _returnvalue_3 (+ _z _speed))
  (if (Variables|Default|GetisMovingDown)
    (CallFunction|MoveInternally (Math|Vector|MakeVector _x _y _returnvalue_2) _returnvalue_2)
    (else
      (CallFunction|MoveInternally (Math|Vector|MakeVector _x _y _returnvalue_3) _returnvalue_3))))

(fn MoveInternally
  (params (NewLocation :type Vector) (Input :type Float%20%28single-precision%29))
  (Math|Float|CompareFloat Input (Variables|Default|GetbottomLimit)
    (:>
      _)
    (:==
      (Variables|Default|SetisMovingDown false :!label _label))
    (:<
      (goto _label)))
  (Math|Float|CompareFloat Input (Variables|Default|GettopLimit)
    (:>
      (bind _asld41player_controller (Utilities|Casting|CastToLD41PlayerController (Game|GetPlayerController 0) :!label _label_2))
      (Variables|/Game/GameLogic/LD41PlayerController.LD41PlayerController_C|SethookActivated _asld41player_controller false))
    (:==
      (goto _label_2))
    (:<
      (Transformation|SetActorLocation NewLocation false false))))