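; Runs the rhythm minigame, spawning arrows from the player controller's timed pattern and showing the points.
; Each tick it slides arrows along -Y at a frame-rate-dependent step and spawns the earliest pattern entry once its time is reached.
; The sphere is the hit zone, publishing the overlapping arrow to FishingGameMode.
; An arrow reaching the static mesh is destroyed and loads TopDownExampleMap to return to stealth mode.
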(event OnComponentBeginOverlap(StaticMesh)
  (params (OverlappedComponent :type Primitive%20Component%20Object%20Reference) (OtherActor :type Actor%20Object%20Reference) (OtherComp :type Primitive%20Component%20Object%20Reference) (OtherBodyIndex :type Integer) (bFromSweep :type Boolean) (SweepResult :type Hit%20Result%20Structure%20%28by%20ref%29))
  (bind _asbp_base_arrow (Utilities|Casting|CastToBP_BaseArrow OtherActor))
  (bind _asfishing_game_mode (Utilities|Casting|CastToFishingGameMode (Game|GetGameMode)))
  (Utilities|Array|RemoveItem (Variables|/Game/GameLogic/FishingGameMode.FishingGameMode_C|GetspawnedElements _asfishing_game_mode) _asbp_base_arrow)
  (Actor|DestroyActor _asbp_base_arrow)
  ;[1 1 1] return to stealth mode
  (Game|OpenLevel(byName) "TopDownExampleMap"))

(event OnComponentEndOverlap(Sphere)
  (params (OverlappedComponent :type Primitive%20Component%20Object%20Reference) (OtherActor :type Actor%20Object%20Reference) (OtherComp :type Primitive%20Component%20Object%20Reference) (OtherBodyIndex :type Integer))
  (Utilities|Casting|CastToBP_BaseArrow OtherActor)
  (bind _asfishing_game_mode (Utilities|Casting|CastToFishingGameMode (Game|GetGameMode)))
  (Variables|/Game/GameLogic/FishingGameMode.FishingGameMode_C|SetoverlappingElement _asfishing_game_mode 0))

(event OnComponentBeginOverlap(Sphere)
  (params (OverlappedComponent :type Primitive%20Component%20Object%20Reference) (OtherActor :type Actor%20Object%20Reference) (OtherComp :type Primitive%20Component%20Object%20Reference) (OtherBodyIndex :type Integer) (bFromSweep :type Boolean) (SweepResult :type Hit%20Result%20Structure%20%28by%20ref%29))
  (bind _asbp_base_arrow (Utilities|Casting|CastToBP_BaseArrow OtherActor))
  (bind _asfishing_game_mode (Utilities|Casting|CastToFishingGameMode (Game|GetGameMode)))
  (Variables|/Game/GameLogic/FishingGameMode.FishingGameMode_C|SetoverlappingElement _asfishing_game_mode _asbp_base_arrow))

(event EventTick
  (params (DeltaSeconds :type Float%20%28single-precision%29))
  (bind _asld41player_controller (Utilities|Casting|CastToLD41PlayerController (Game|GetPlayerController 0)))
  (Rendering|Components|TextRender|SetText (Variables|Default|GetTextRender) (Utilities|Text|ToText(Integer) (Variables|/Game/GameLogic/LD41PlayerController.LD41PlayerController_C|GetPoints _asld41player_controller)))
  (CallFunction|UpdateElements)
  (bind _output_get (Variables|/Game/GameLogic/LD41PlayerController.LD41PlayerController_C|SetcurrentRhythmSectionTime _asld41player_controller (+ (Variables|/Game/GameLogic/LD41PlayerController.LD41PlayerController_C|GetcurrentRhythmSectionTime _asld41player_controller) DeltaSeconds)))
  (Math|Integer|CompareInt (Utilities|Map|Length (Variables|/Game/GameLogic/LD41PlayerController.LD41PlayerController_C|GetcurrentPattern _asld41player_controller))
    (:>
      (bind _keys (Utilities|Map|Keys (Variables|/Game/GameLogic/LD41PlayerController.LD41PlayerController_C|GetcurrentPattern _asld41player_controller)))
      (Math|Float|CompareFloat _output_get (Utilities|Array|Get(acopy) _keys (.IndexOfMinValue (Math|Float|MinOfFloatArray _keys)))
        (:>
          _)
        (:==
          _))
      (bind _values (Utilities|Map|Values (Variables|/Game/GameLogic/LD41PlayerController.LD41PlayerController_C|GetcurrentPattern _asld41player_controller)))
      (CallFunction|AddPatternElementtoScreen (Utilities|Array|Get(acopy) _values (.IndexOfMinValue (Math|Float|MinOfFloatArray _keys))))
      (Utilities|Map|Remove (Variables|/Game/GameLogic/LD41PlayerController.LD41PlayerController_C|GetcurrentPattern _asld41player_controller) (Utilities|Array|Get(acopy) _keys (.IndexOfMinValue (Math|Float|MinOfFloatArray _keys)))))))

(fn ConstructionScript)

(fn AddPatternElementtoScreen
  (params (element :type E_PatternElements%20Enum :default "NewEnumerator0"))
  (bind _returnvalue (Math|Transform|MakeTransform "69.500000,35.000000,0.000000" "0.000000,90.000000,0.000000"))
  (bind _asfishing_game_mode (Utilities|Casting|CastToFishingGameMode (Game|GetGameMode)))
  (switch Utilities|FlowControl|Switch|SwitchonE_PatternElements element
    (:NewEnumerator0
      (bind _returnvalue_2 (Game|SpawnActorfromClass "/Game/GameLogic/BP_UpArrow.BP_UpArrow_C" _returnvalue "Undefined" 0 0))
      (Utilities|Array|Add (Variables|/Game/GameLogic/FishingGameMode.FishingGameMode_C|GetspawnedElements _asfishing_game_mode) _returnvalue_2))
    (:NewEnumerator1
      (bind _returnvalue_3 (Game|SpawnActorfromClass "/Game/GameLogic/BP_DownArrow.BP_DownArrow_C" _returnvalue "Undefined" 0 0))
      (Variables|/Game/GameLogic/BP_BaseArrow.BP_BaseArrow_C|Setelement _returnvalue_3 "NewEnumerator1")
      (Utilities|Array|Add (Variables|/Game/GameLogic/FishingGameMode.FishingGameMode_C|GetspawnedElements _asfishing_game_mode) _returnvalue_3))
    (:NewEnumerator2
      (bind _returnvalue_4 (Game|SpawnActorfromClass "/Game/GameLogic/BP_LEftArrow.BP_LeftArrow_C" _returnvalue "Undefined" 0 0))
      (Variables|/Game/GameLogic/BP_BaseArrow.BP_BaseArrow_C|Setelement _returnvalue_4 "NewEnumerator2")
      (Utilities|Array|Add (Variables|/Game/GameLogic/FishingGameMode.FishingGameMode_C|GetspawnedElements _asfishing_game_mode) _returnvalue_4))
    (:NewEnumerator3
      (bind _returnvalue_5 (Game|SpawnActorfromClass "/Game/GameLogic/BP_RightArrow.BP_RightArrow_C" _returnvalue "Undefined" 0 0))
      (Variables|/Game/GameLogic/BP_BaseArrow.BP_BaseArrow_C|Setelement _returnvalue_5 "NewEnumerator3")
      (Utilities|Array|Add (Variables|/Game/GameLogic/FishingGameMode.FishingGameMode_C|GetspawnedElements _asfishing_game_mode) _returnvalue_5))))

(fn UpdateElements
  (bind _asfishing_game_mode (Utilities|Casting|CastToFishingGameMode (Game|GetGameMode)))
  (for _array_element (Variables|/Game/GameLogic/FishingGameMode.FishingGameMode_C|GetspawnedElements _asfishing_game_mode)
    (Transformation|SetActorLocation _array_element (Math|Vector|MakeVector (.X (Math|Vector|BreakVector (Transformation|GetActorLocation _array_element))) (- (.Y (Math|Vector|BreakVector (Transformation|GetActorLocation _array_element))) (Variables|Default|GetelementSpeed)) (.Z (Math|Vector|BreakVector (Transformation|GetActorLocation _array_element)))) false false)))

(fn SetupRhythmSection
  (bind _asfishing_game_mode (Utilities|Casting|CastToFishingGameMode (Game|GetGameMode)))
  (Variables|/Game/GameLogic/FishingGameMode.FishingGameMode_C|SetcollisionCenter _asfishing_game_mode (Transformation|GetWorldLocation (Variables|Default|GetSphere))))