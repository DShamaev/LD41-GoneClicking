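; BP_HiddenArrow is a Blueprint that holds a randomly chosen music pattern, apparently the hidden answer that an arrow's pattern is checked against.
; Setup picks one of four E_MusicPattern values at random by casting a random integer to the enum, and stores it in Pattern.
; CheckPattern returns whether a supplied arrow pattern equals the stored one.
; The event graph and construction script add no behavior of their own.
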(event EventBeginPlay
  (|CallParentFunction) ; This node is disabled and will not be called.\nDrag off pins to build functionality.
)

(event Collision|EventActorBeginOverlap
  (params (OtherActor :type Actor%20Object%20Reference))
  (|CallParentFunction OtherActor) ; This node is disabled and will not be called.\nDrag off pins to build functionality.
)

(event EventTick
  (params (DeltaSeconds :type Float%20%28single-precision%29))
  (|CallParentFunction DeltaSeconds) ; This node is disabled and will not be called.\nDrag off pins to build functionality.
)

(fn ConstructionScript
  (|CallParentFunction))

(fn Setup
  (Variables|Default|Setpattern (Utilities|Enum|ByteToEnumE_MusicPattern (Math|Conversions|ToByte(Integer) (Math|Random|RandomIntegerinRange 0 3)))))

(fn CheckPattern
  (params (arrowPAttern :type E_MusicPattern%20Enum :default "NewEnumerator0"))
  (return (Utilities|Enum|Equal(Enum) arrowPAttern (Variables|Default|Getpattern))))